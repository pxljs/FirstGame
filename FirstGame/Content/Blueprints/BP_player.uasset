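; Player character Blueprint with Enhanced Input movement and look, a melee attack and health.
; On BeginPlay it adds the input mapping, fills health and shows health bar and HUD widgets.
; Attacks play a push montage gated by CanAttack, with notifies triggering a forward sphere trace that damages pawns.
; Taking damage triggers HUD and sound feedback, then either knockback or, at zero health, disabled input and ragdoll.
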(event `self.ReceiveBeginPlay`
  ;[0.09549 0.09549 0.09549] Input
  (`EnhancedInputSubsystemInterface.AddMappingContext` (pcsubsystem `EnhancedInputLocalPlayerSubsystem` (`GameplayStatics.GetPlayerController` 0)) "/Game/Input/IMC_PlayerInput.IMC_PlayerInput" 0 (struct))
  (set `self.Health` (`self.Max Health`))
  (bind _returnvalue (`|CreateWidget` "/Game/UI/WB_HealthBar.WB_HealthBar_C"))
  (`UserWidget.AddToViewport` _returnvalue 0)
  (bind _returnvalue_2 (`|CreateWidget` "/Game/UI/WB_HUD.WB_HUD_C"))
  (bind _output_get (set `self.HUD Widget` _returnvalue_2))
  (`UserWidget.AddToViewport` _output_get 0))

(event `EnhancedInput|/Game/Input/IA_Move`
  (params (ActionValue :type "Vector2D Structure") (ElapsedSeconds :type "Float (double-precision)") (TriggeredSeconds :type "Float (double-precision)") (InputAction :type "InputAction Object Reference" :default "/Game/Input/IA_Move.IA_Move"))
  (bind (_returnvalue_roll _returnvalue_pitch _returnvalue_yaw) (`KismetMathLibrary.BreakRotator` (`self.GetControlRotation`)))
  (bind (_returnvalue_roll_2 _returnvalue_pitch_2 _returnvalue_yaw_2) (`KismetMathLibrary.BreakRotator` (`self.GetControlRotation`)))
  ;[0.09549 0.09549 0.09549] Movement
  (:`Triggered`
    (`self.AddMovementInput` (`KismetMathLibrary.GetRightVector` (`KismetMathLibrary.MakeRotator` _returnvalue_roll 0.0 _returnvalue_yaw)) ActionValue_X)
    (`self.AddMovementInput` (`KismetMathLibrary.GetForwardVector` (`KismetMathLibrary.MakeRotator` _returnvalue_roll_2 0.0 _returnvalue_yaw_2)) ActionValue_Y)))

(event `EnhancedInput|/Game/Input/IA_Look`
  (params (ActionValue :type "Vector2D Structure") (ElapsedSeconds :type "Float (double-precision)") (TriggeredSeconds :type "Float (double-precision)") (InputAction :type "InputAction Object Reference" :default "/Game/Input/IA_Look.IA_Look"))
  ;[0.09549 0.09549 0.09549] Movement
  (:`Triggered`
    (`self.AddControllerYawInput` ActionValue_X)
    (`self.AddControllerPitchInput` (* ActionValue_Y -1.0))))

(event `EnhancedInput|/Game/Input/IA_Attack`
  (params (ActionValue :type Boolean) (ElapsedSeconds :type "Float (double-precision)") (TriggeredSeconds :type "Float (double-precision)") (InputAction :type "InputAction Object Reference" :default "/Game/Input/IA_Attack.IA_Attack"))
  (bind _attack_trace_pos (`self.Attack Trace Pos`))
  (bind _returnvalue (`SceneComponent.K2_GetComponentLocation` _attack_trace_pos))
  (:`Started`
    (if (`self.Can Attack`)
      (`|PlayMontage` (`self.Mesh`) "/Game/Characters/Mannequin_UE4/OurAnimations/Push_Montage.Push_Montage"
        (:`then`
          (set `self.Can Attack` false))
        (:`OnCompleted`
          (set `self.Can Attack` true))
        (:`OnNotifyBegin`
          (bind (_outhit _returnvalue_2) (`KismetSystemLibrary.SphereTraceSingleForObjects` _returnvalue (+ _returnvalue (* (`SceneComponent.GetForwardVector` _attack_trace_pos) 100.0)) 30.0 (`|MakeArray` "ObjectTypeQuery3" :!type "EObjectTypeQuery Enum")))
          (if _returnvalue_2
            (`GameplayStatics.ApplyDamage` (`.HitActor` (`GameplayStatics.BreakHitResult` _outhit)) 10.0)))))))

(event `self.ReceiveAnyDamage`
  (params (Damage :type "Float (single-precision)") (DamageType :type "DamageType Object Reference") (InstigatedBy :type "Controller Object Reference") (DamageCauser :type "Actor Object Reference"))
  (set `self.Health` (- (`self.Health`) Damage))
  (`/Game/UI/WB_HUD.Damage Screen` (`self.HUD Widget`))
  (`GameplayStatics.PlaySoundAtLocation` "/Game/Audio/MS_DamageGrunt.MS_DamageGrunt" (`self.K2_GetActorLocation`) (struct) 1.0 1.0 0.0 null null null null)
  (if (<= (`self.Health`) 0.0)
    (`self.DisableInput` null)
    (`PrimitiveComponent.SetSimulatePhysics` (`self.Mesh`) true)
    (else
      (`self.LaunchCharacter` (+ (* (`self.GetActorForwardVector`) -200.0) (* (`self.GetActorUpVector`) 100.0))))))

(fn `UserConstructionScript`)